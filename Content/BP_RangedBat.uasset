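; BP_RangedBat is a bat enemy, a child Blueprint that adds hit feedback and flapping audio to its parent's behavior.
; On BeginPlay it creates dynamic materials for both bat mesh slots and attaches a looping-style flap sound.
; Damage triggers a timeline driving the HitEffect material parameter, then defers to the parent.
; The death-like GaDoodTyfus override pauses the sound, and Stop pauses or resumes it with its flag.
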(event `self.ReceiveBeginPlay`
  (bind _bat (`self.bat`))
  (bind _bat_2 (`self.bat`))
  (`parent.ReceiveBeginPlay`)
  (bind _returnvalue (`PrimitiveComponent.CreateDynamicMaterialInstance` _bat 0 (`PrimitiveComponent.GetMaterial` _bat_2 0) "None"))
  (set `self.Mat` _returnvalue)
  (bind _returnvalue_2 (`PrimitiveComponent.CreateDynamicMaterialInstance` _bat 1 (`PrimitiveComponent.GetMaterial` _bat_2 1) "None"))
  (set `self.Mat2` _returnvalue_2)
  (bind _returnvalue_3 (`GameplayStatics.SpawnSoundAttached` "/Game/Audio/SoundEffects/batflap.batflap" (`self.Mesh`) "None" (0.0 0.0 0.0) (struct) "KeepRelativeOffset" false 1.0 1.0 0.0 null null))
  (set `self.Audio` _returnvalue_3))

(event `HitEffect`
  (bind _mat (`self.Mat`)
    (:`then`
      (bind _mat2 (`self.Mat2`)
        (:`then`
          (bind (_direction _curve) (`Timeline|Timeline` :!via `PlayFromStart`)
            (:`Update`
              (`MaterialInstanceDynamic.SetScalarParameterValue` _mat "HitEffect" _curve)
              (`MaterialInstanceDynamic.SetScalarParameterValue` _mat2 "HitEffect" _curve))))
        (:`else`)))
    (:`else`)))

(fn `Damage`
  (params (Amt :type "Float (double-precision)") (Normal :type "Vector Structure"))
  (returns (Dead :type Boolean))
  (`self.HitEffect`)
  (bind _dead (`parent.Damage` Amt Normal))
  (return _dead))

(fn `GaDoodTyfus`
  (`parent.GaDoodTyfus`)
  (`AudioComponent.SetPaused` (`self.audio`) true))

(fn `stop`
  (params (dn :type Boolean))
  (`parent.stop` dn)
  (`AudioComponent.SetPaused` (`self.Audio`) dn))

(fn `UserConstructionScript`
  (`parent.UserConstructionScript`))