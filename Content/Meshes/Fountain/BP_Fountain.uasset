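; BP_Fountain is a healing fountain that restores BP_ThirdPersonCharacter to full health on interaction.
; Entering its box shows the "Fountain" dialogue above it through BP_DialogueManager if the character's CanUseFountain is set, and leaving clears it.
; Interact sets Health to MaxHealth, calls UpdateHealth and adds a Niagara effect, without rechecking CanUseFountain.
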(event `self.Box.OnComponentBeginOverlap`
  (params (OverlappedComponent :type "PrimitiveComponent Object Reference") (OtherActor :type "Actor Object Reference") (OtherComp :type "PrimitiveComponent Object Reference") (OtherBodyIndex :type Integer) (bFromSweep :type Boolean) (SweepResult :type "HitResult Structure (by ref)"))
  (bind _asbp_third_person_character (cast `/Game/ThirdPerson/Blueprints/BP_ThirdPersonCharacter` OtherActor))
  (if (`/Game/ThirdPerson/Blueprints/BP_ThirdPersonCharacter.canUseFountain` _asbp_third_person_character)
    (bind _returnvalue (`GameplayStatics.GetActorOfClass` "/Game/Blueprints/BP_DialogueManager.BP_DialogueManager_C"))
    (`/Engine/EditorBlueprintResources/StandardMacros.IsValid` _returnvalue
      (:`Is Valid`
        (`/Game/Blueprints/BP_DialogueManager.TriggerDialogue` _returnvalue "Fountain" -1 self (0.0 0.0 300.0))))))

(event `self.Box.OnComponentEndOverlap`
  (params (OverlappedComponent :type "PrimitiveComponent Object Reference") (OtherActor :type "Actor Object Reference") (OtherComp :type "PrimitiveComponent Object Reference") (OtherBodyIndex :type Integer))
  (cast `/Game/ThirdPerson/Blueprints/BP_ThirdPersonCharacter` OtherActor)
  (bind _returnvalue (`GameplayStatics.GetActorOfClass` "/Game/Blueprints/BP_DialogueManager.BP_DialogueManager_C"))
  (`/Engine/EditorBlueprintResources/StandardMacros.IsValid` _returnvalue
    (:`Is Valid`
      (`/Game/Blueprints/BP_DialogueManager.ClearDialogue` _returnvalue))))

(event `/Game/Blueprints/I_Interactable.Interact`
  (params (Interactor :type "Character Object Reference"))
  (bind _asbp_third_person_character (cast `/Game/ThirdPerson/Blueprints/BP_ThirdPersonCharacter` Interactor))
  (set `/Game/ThirdPerson/Blueprints/BP_ThirdPersonCharacter.Health` (`/Game/ThirdPerson/Blueprints/BP_ThirdPersonCharacter.MaxHealth` _asbp_third_person_character) _asbp_third_person_character)
  (`/Game/ThirdPerson/Blueprints/BP_ThirdPersonCharacter.UpdateHealth` _asbp_third_person_character)
  (`AddComponent|NODE_AddNiagaraComponent-0`))

(fn `UserConstructionScript`)