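; BP_Spawn is an actor that plays a spawn effect for the player character when play begins, or through its SpawnDemon event.
; The ShowAmount timeline drives two Niagara systems' User.ShowAmount and the Z lift of a stand-in skeletal mesh.
; On finish, it zeroes both effects, hides the stand-in, reveals the player's mesh and enables CanMove.
; An added Niagara effect is destroyed after a delay.
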(event `SpawnDemon`
  (bind (_direction _showamount _liftcharacter) (`Timeline|ShowAmount` :!via `PlayFromStart` :!label _label)
    (:`Update`
      (`NiagaraComponent.SetVariableFloat` (`self.NS_SpawnSmoke`) "User.ShowAmount" _showamount)
      (`NiagaraComponent.SetVariableFloat` (`self.NS_Spawn`) "User.ShowAmount" _showamount)
      (`SceneComponent.K2_SetRelativeLocation` (`self.SkeletalMesh`) (`KismetMathLibrary.MakeVector` 0.0 0.0 _liftcharacter) false false))
    (:`Finished`
      (`NiagaraComponent.SetVariableFloat` (`self.NS_SpawnSmoke`) "User.ShowAmount" 0.0)
      (`NiagaraComponent.SetVariableFloat` (`self.NS_Spawn`) "User.ShowAmount" 0.0)
      (bind _returnvalue (`AddComponent|NODE_AddNiagaraComponent-0`))
      (`SceneComponent.SetVisibility` (`self.SkeletalMesh`) false false)
      (`|ExecutionSequence`
        (:`then_0`
          (bind _asbp_third_person_character (cast `/Game/ThirdPerson/Blueprints/BP_ThirdPersonCharacter` (`GameplayStatics.GetPlayerCharacter` 0)))
          (`SceneComponent.SetHiddenInGame` (`Character.Mesh` _asbp_third_person_character) false true)
          (set `/Game/ThirdPerson/Blueprints/BP_ThirdPersonCharacter.canMove` true _asbp_third_person_character))
        (:`then_1`
          (`KismetSystemLibrary.Delay` 5.0)
          (`ActorComponent.K2_DestroyComponent` _returnvalue))))))

(event `self.ReceiveBeginPlay`
  (goto _label :!via `PlayFromStart`))

(fn `UserConstructionScript`)