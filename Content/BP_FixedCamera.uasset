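; BP_FixedCamera is a camera actor that trails the player within a bounded area at a fixed height.
; It caches the player character on BeginPlay, then each Tick lerps toward the player's location plus an offset, with delta time scaling the smoothing.
; X and Y are clamped to min/max limits, while Z is set directly to the offset's Z, ignoring the player's height.
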(event `self.ReceiveBeginPlay`
  ;[1 1 1] Event - BeginPlay
  (set `self.Player` (`GameplayStatics.GetPlayerCharacter` 0)))

(event `self.ReceiveTick`
  (params (DeltaSeconds :type "Float (single-precision)"))
  (bind (_offset_x _offset_y _offset_z) (`KismetMathLibrary.BreakVector` (`self.Offset`)))
  (bind (_returnvalue_x _returnvalue_y _returnvalue_z) (`KismetMathLibrary.BreakVector` (`KismetMathLibrary.VLerp` (`self.K2_GetActorLocation`) (+ (`self.K2_GetActorLocation` (`self.Player`)) (`self.Offset`)) (* DeltaSeconds 2.0))))
  ;[1 1 1] Event - Tick
  (`self.K2_SetActorLocationAndRotation` (`KismetMathLibrary.MakeVector` (`KismetMathLibrary.FClamp` _returnvalue_x (`self.MinX`) (`self.MaxX`)) (`KismetMathLibrary.FClamp` _returnvalue_y (`self.MinY`) (`self.MaxY`)) _offset_z)))

(fn `UserConstructionScript`)