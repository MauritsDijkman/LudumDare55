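; BP_UselessWizard is a wizard actor that reacts to being hit with dialogue instead of taking damage.
; Tick sways its static mesh with a time-based sine on relative X and Z, mostly as a vertical bob.
; Damage finds BP_DialogueManager, triggers one of three random MageHit lines with an offset above itself, and returns false.
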(event `self.ReceiveTick`
  (params (DeltaSeconds :type "Float (single-precision)"))
  (bind _returnvalue (`KismetMathLibrary.Sin` (`GameplayStatics.GetTimeSeconds`)))
  (`SceneComponent.K2_SetRelativeLocation` (`self.StaticMesh`) (`KismetMathLibrary.MakeVector` _returnvalue 0.0 (* _returnvalue 5.0)) false false))

(fn `Damage`
  (params (Amt :type "Float (double-precision)") (Normal :type "Vector Structure"))
  (returns (Dead :type Boolean))
  (bind _returnvalue (`GameplayStatics.GetActorOfClass` "/Game/Blueprints/BP_DialogueManager.BP_DialogueManager_C"))
  (`/Engine/EditorBlueprintResources/StandardMacros.IsValid` _returnvalue
    (:`Is Valid`
      (`/Game/Blueprints/BP_DialogueManager.TriggerDialogue` _returnvalue (`KismetStringLibrary.Concat_StrStr` "MageHit" (`KismetStringLibrary.Conv_IntToString` (`KismetMathLibrary.RandomIntegerInRange` 0 2))) -1 self (0.0 0.0 300.0))
      (return false))))

(fn `UserConstructionScript`)