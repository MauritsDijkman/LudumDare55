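; Base throwable projectile that launches at a velocity set by Init and explodes on contact, ignoring overlaps with its instigator's class.
; Overlaps send BPI_Damagable damage, optionally slowing Characters.
; Overlaps and blocking hits share the explosion path: Niagara effects, camera shake, sound, stopping the flame loop, removing collision and delayed despawn.
; OnHit and OnExplode are empty hooks, apparently for child throwables.
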(event `self.ReceiveBeginPlay`
  (bind _returnvalue (`GameplayStatics.SpawnSoundAttached` "/Game/Audio/SoundEffects/flame.flame" (`self.Sphere`) "None" (0.0 0.0 0.0) (struct) "KeepRelativeOffset" true 1.0 (`KismetMathLibrary.RandomFloatInRange` 0.95 1.05) 0.0 null null))
  (set `self.flame` _returnvalue))

(event `self.Sphere.OnComponentBeginOverlap`
  (params (OverlappedComponent :type "PrimitiveComponent Object Reference") (OtherActor :type "Actor Object Reference") (OtherComp :type "PrimitiveComponent Object Reference") (OtherBodyIndex :type Integer) (bFromSweep :type Boolean) (SweepResult :type "HitResult Structure (by ref)"))
  ;[1 1 1] Pawn
  (if (!= (`GameplayStatics.GetObjectClass` OtherActor) (`GameplayStatics.GetObjectClass` (`self.Instigator`)))
    (if (`KismetSystemLibrary.DoesImplementInterface` OtherActor "/Game/Blueprints/BPI_Damagable.BPI_Damagable_C")
      (message `/Game/Blueprints/BPI_Damagable.Damage` OtherActor (`self.Damage`) (* (`KismetMathLibrary.Normal` (- (`self.K2_GetActorLocation`) (`self.K2_GetActorLocation`))) (`self.knockbackMultiplier`)))
      (bind _ascharacter (cast `Character` OtherActor)
        (:`then`
          (`self.OnHit` _ascharacter)
          (if (`self.slowsEnemy`)
            (bind _charactermovement (`Character.CharacterMovement` _ascharacter))
            (set `CharacterMovementComponent.MaxWalkSpeed` (* (`CharacterMovementComponent.MaxWalkSpeed` _charactermovement) 0.7) _charactermovement)))
        (:`CastFailed`
          _))
      ;[1 1 1] Environment
      (`self.SpawnNiagra` (`self.Explosion Color`) (`self.Explosion Size`) :!label _label)
      (bind _returnvalue (`GameplayStatics.GetActorOfClass` "/Game/Blueprints/BP_FixedCamera.BP_FixedCamera_C"))
      (`/Game/Blueprints/BP_FixedCamera.ShakeCamera` _returnvalue 1.0)
      (`self.OnExplode`)
      (`NiagaraComponent.SetVariableBool` (`self.Niagara`) "User.Hit" true)
      (`GameplayStatics.PlaySoundAtLocation` "/Game/Audio/SoundEffects/bigfireball.bigfireball" (`self.K2_GetActorLocation`) (struct) 1.0 (`KismetMathLibrary.SelectFloat` 0.95 1.05) 0.0 null null null null)
      (bind _flame (`self.flame`)
        (:`then`
          (`AudioComponent.Stop` _flame))
        (:`else`
          _))
      (`ActorComponent.K2_DestroyComponent` (`self.Sphere`))
      (`self.SetLifeSpan` 2.0))))

(event `self.Sphere.OnComponentHit`
  (params (HitComponent :type "PrimitiveComponent Object Reference") (OtherActor :type "Actor Object Reference") (OtherComp :type "PrimitiveComponent Object Reference") (NormalImpulse :type "Vector Structure") (Hit :type "HitResult Structure (by ref)"))
  ;[1 1 1] Environment
  (goto _label))

(fn `Init`
  (params (LaunchVelociy :type "Vector Structure"))
  (bind _projectilemovement (`self.ProjectileMovement`))
  (set `self.Launch Velociy` LaunchVelociy)
  (set `MovementComponent.Velocity` LaunchVelociy _projectilemovement)
  (set `ProjectileMovementComponent.bRotationFollowsVelocity` true _projectilemovement))

(fn `OnExplode`)

(fn `OnHit`
  (params (Target :type "Character Object Reference") (ExplosionSIze :type "Float (double-precision)") (ExplosionColor :type "LinearColor Structure")))

(fn `SpawnNiagra`
  (params (`Explosion Color` :type "LinearColor Structure") (`Explosion Size` :type "Float (double-precision)"))
  (bind _returnvalue (`AddComponent|NODE_AddNiagaraComponent-0`))
  (`NiagaraComponent.SetVariableFloat` _returnvalue "User.Size" `Explosion Size`)
  (`NiagaraComponent.SetVariableLinearColor` _returnvalue "User.Color" `Explosion Color`))

(fn `UserConstructionScript`)