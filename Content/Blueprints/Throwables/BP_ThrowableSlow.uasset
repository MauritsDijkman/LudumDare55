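; Throwable projectile that damages what it overlaps and scales a third-person character's max walk speed by a multiplier, with no restore here.
; Init lobs it at a target using a suggested toss velocity, leading the target's movement by estimated flight time, with launch speed scaled by a distance-driven curve.
; Character overlaps and any blocking hit spawn a Niagara effect flagged as hit, remove the collision sphere and set a short lifespan.
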(event `self.Sphere.OnComponentBeginOverlap`
  (params (OverlappedComponent :type "PrimitiveComponent Object Reference") (OtherActor :type "Actor Object Reference") (OtherComp :type "PrimitiveComponent Object Reference") (OtherBodyIndex :type Integer) (bFromSweep :type Boolean) (SweepResult :type "HitResult Structure (by ref)"))
  ;[1 1 1] Pawn
  (bind _asbpi_damagable (cast `/Game/Blueprints/BPI_Damagable` OtherActor))
  (`/Game/Blueprints/BPI_Damagable.Damage` _asbpi_damagable (`self.Damage`) (`KismetMathLibrary.Normal` (- (`self.K2_GetActorLocation`) (`self.K2_GetActorLocation`))))
  ;[1 1 1] Set Max Walking Speed
  (bind _asbp_third_person_character (cast `/Game/ThirdPerson/Blueprints/BP_ThirdPersonCharacter` OtherActor))
  (bind _charactermovement (`Character.CharacterMovement` _asbp_third_person_character))
  (set `CharacterMovementComponent.MaxWalkSpeed` (* (`CharacterMovementComponent.MaxWalkSpeed` _charactermovement) (`self.Max Speed Multiplier`)) _charactermovement)
  ;[1 1 1] Niagra
  (`self.SpawnNiagra` :!label _label)
  (`NiagaraComponent.SetVariableBool` (`self.Niagara`) "User.Hit" true)
  (`ActorComponent.K2_DestroyComponent` (`self.Sphere`))
  (`self.SetLifeSpan` 2.0))

(event `self.Sphere.OnComponentHit`
  (params (HitComponent :type "PrimitiveComponent Object Reference") (OtherActor :type "Actor Object Reference") (OtherComp :type "PrimitiveComponent Object Reference") (NormalImpulse :type "Vector Structure") (Hit :type "HitResult Structure (by ref)"))
  ;[1 1 1] Environment
  (goto _label))

(fn `Init`
  (params (AttackTarget :type "Actor Object Reference"))
  (locals (LV_AttackTarget :type "Actor Object Reference") (LV_Player_Z_Offset :type "Float (double-precision)" :default 0.0) (LV_ProjectileSpeed :type "Float (double-precision)" :default 1000.0) (LV_Curve :type "CurveFloat Object Reference" :default "/Script/Engine.CurveFloat'/Game/Blueprints/ProjectileSpeed.ProjectileSpeed'"))
  (bind _lv_attacktarget (`local.LV_AttackTarget`))
  (bind _projectilemovement (`self.ProjectileMovement`))
  (bind (_returnvalue_x _returnvalue_y _returnvalue_z) (`KismetMathLibrary.BreakVector` (`self.K2_GetActorLocation` _lv_attacktarget)))
  (bind _returnvalue (`self.GetDistanceTo` _lv_attacktarget))
  (bind _returnvalue_2 (* (`CurveFloat.GetFloatValue` (`local.LV_Curve`) (`KismetMathLibrary.MapRangeClamped` _returnvalue 200.0 1500.0 0.0 1.0)) (`local.LV_ProjectileSpeed`)))
  (set `local.LV_AttackTarget` AttackTarget)
  (`/Engine/EditorBlueprintResources/StandardMacros.IsValid` _lv_attacktarget
    (:`Is Valid`
      (bind _tossvelocity (`GameplayStatics.BlueprintSuggestProjectileVelocity` (`self.K2_GetActorLocation`) (+ (`KismetMathLibrary.MakeVector` _returnvalue_x _returnvalue_y (+ _returnvalue_z (`local.LV_Player_Z_Offset`))) (* (/ _returnvalue _returnvalue_2) (`self.GetVelocity` _lv_attacktarget))) _returnvalue_2 0.0 "DoNotTrace"))
      (set `MovementComponent.Velocity` _tossvelocity _projectilemovement)
      (set `ProjectileMovementComponent.bRotationFollowsVelocity` true _projectilemovement))))

(fn `SpawnNiagra`
  (`AddComponent|NODE_AddNiagaraComponent-0`))

(fn `UserConstructionScript`)