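; BP_Wall is a brick wall actor with pillars, collision control and links to the doors overlapping it.
; The construction script uses SeeThru to switch to back-wall materials and disable shadow casting.
; On BeginPlay or BindDoors, it caches BP_BasicDoor actors overlapping DoorCheck, which SetDoorVisible shows or hides along with their collision.
; GetRandomDoorPos returns a random point along the right vector within one of two spans.
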(event `Bind Doors`
  (`KismetArrayLibrary.Array_Clear` (`self.Door`) :!label _label)
  (for _array_element (`PrimitiveComponent.GetOverlappingActors` (`self.DoorCheck`) "/Game/Blueprints/BP_BasicDoor.BP_BasicDoor_C")
    (bind _asbp_basic_door (cast `/Game/Blueprints/BP_BasicDoor` _array_element))
    (`KismetArrayLibrary.Array_Add` (`self.Door`) _asbp_basic_door)))

(event `self.ReceiveBeginPlay`
  (goto _label))

(fn `GetRandomDoorPos`
  (returns (Pos :type "Vector Structure"))
  (locals (RanVar :type Boolean :default false))
  (bind _ranvar (`local.RanVar`))
  (set `local.RanVar` (`KismetMathLibrary.RandomBool`))
  (return (+ (`self.K2_GetActorLocation`) (* (`KismetMathLibrary.RandomFloatInRange` (`KismetMathLibrary.SelectFloat` 200.0 1000.0 _ranvar) (`KismetMathLibrary.SelectFloat` 550.0 1350.0 _ranvar)) (`self.GetActorRightVector`)))))

(fn `SetDoorVisible`
  (params (Visible :type Boolean))
  (for _array_element (`self.Door`)
    (`self.SetActorHiddenInGame` _array_element (not Visible))
    (`PrimitiveComponent.SetCollisionEnabled` (`/Game/Blueprints/BP_BasicDoor.DoorGFX` _array_element) (select `bool` Visible :`false` "NoCollision" :`true` "QueryAndPhysics" :!type "ECollisionEnabled Enum"))))

(fn `SetWallCollision`
  (params (NewType :type "ECollisionEnabled Enum" :default "NoCollision"))
  (`PrimitiveComponent.SetCollisionEnabled` (`self.Wall_01`) NewType)
  (`PrimitiveComponent.SetCollisionEnabled` (`self.Wall_02`) NewType)
  (`PrimitiveComponent.SetCollisionEnabled` (`self.Wall_03`) NewType)
  (`PrimitiveComponent.SetCollisionEnabled` (`self.Wall_04`) NewType))

(fn `UserConstructionScript`
  (bind _seethru (`self.SeeThru`))
  (`PrimitiveComponent.SetMaterial` (`self.Wall_03`) 0 (select `bool` _seethru :`false` "/Game/Meshes/Walls/M_Bricks.M_Bricks" :`true` "/Game/Meshes/Walls/M_BricksBackWall.M_BricksBackWall" :!type "MaterialInterface Object Reference"))
  (`PrimitiveComponent.SetMaterial` (`self.Wall_02`) 0 (select `bool` _seethru :`false` "/Game/Meshes/Walls/M_Bricks.M_Bricks" :`true` "/Game/Meshes/Walls/M_BricksBackWall.M_BricksBackWall" :!type "MaterialInterface Object Reference"))
  (`PrimitiveComponent.SetMaterial` (`self.Wall_04`) 0 (select `bool` _seethru :`false` "/Game/Meshes/Walls/M_Bricks.M_Bricks" :`true` "/Game/Meshes/Walls/M_BricksBackWall.M_BricksBackWall" :!type "MaterialInterface Object Reference"))
  (`PrimitiveComponent.SetMaterial` (`self.Wall_01`) 0 (select `bool` _seethru :`false` "/Game/Meshes/Walls/M_Bricks.M_Bricks" :`true` "/Game/Meshes/Walls/M_BricksBackWall.M_BricksBackWall" :!type "MaterialInterface Object Reference"))
  (`PrimitiveComponent.SetMaterial` (`self.Pillar_03`) 0 (select `bool` _seethru :`false` "/Game/Meshes/Pillar/M_Pillar.M_Pillar" :`true` "/Game/Meshes/Pillar/M_PillarBackWall.M_PillarBackWall" :!type "MaterialInterface Object Reference"))
  (`PrimitiveComponent.SetMaterial` (`self.Pillar_01`) 0 (select `bool` _seethru :`false` "/Game/Meshes/Pillar/M_Pillar.M_Pillar" :`true` "/Game/Meshes/Pillar/M_PillarBackWall.M_PillarBackWall" :!type "MaterialInterface Object Reference"))
  (`PrimitiveComponent.SetCastShadow` (`self.Wall_03`) (not (`self.SeeThru`)))
  (`PrimitiveComponent.SetCastShadow` (`self.Wall_02`) (not (`self.SeeThru`)))
  (`PrimitiveComponent.SetCastShadow` (`self.Pillar_01`) (not (`self.SeeThru`)))
  (`PrimitiveComponent.SetCastShadow` (`self.Pillar_03`) (not (`self.SeeThru`)))
  (`PrimitiveComponent.SetCastShadow` (`self.Wall_04`) (not (`self.SeeThru`)))
  (`PrimitiveComponent.SetCastShadow` (`self.Wall_01`) (not (`self.SeeThru`))))