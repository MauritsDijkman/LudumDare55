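; BP_DialogueManager is an actor that shows multi-line dialogue in a WBP_Dialogue widget component positioned at the dialogue's instigator.
; TriggerDialogue looks up an entry in Dialogues by identifier or index, moves the actor to the instigator plus an offset, and displays the first colored line.
; ProceedDialogue advances lines, then clears the text, restoring player movement if that dialogue disallowed it.
; DelaySetVisibility is an empty stub, with widget hiding logic left disconnected.
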(event `self.ReceiveBeginPlay`
  (bind _aswbp_dialogue (cast `/Game/Blueprints/Widget/WBP_Dialogue` (`WidgetComponent.GetWidget` (`self.Widget`))))
  (set `self.DialogueWidget` _aswbp_dialogue))

(event `DelaySetVisibility`
  (params (Visible :type Boolean)))

(fn `ClearDialogue`
  (`/Game/Blueprints/Widget/WBP_Dialogue.SetText` :`self` (`self.DialogueWidget`))
  (set `self.CurrentDialogue` (struct))
  (set `self.CurrentLineIndex` 0)
  (set `self.inDialogue` false))

(fn `FindDialogueByID`
  (params (Identifier :type String))
  (returns (`Out Dialogue` :type "/Game/Blueprints/Dialogue Structure") (Success :type Boolean))
  (for _array_element (`self.Dialogues`)
    (if (== (`.Identifier_3_5153007F4C7986772981EF95180469C5` (break `/Game/Blueprints/Dialogue` _array_element)) Identifier)
      (return _array_element true)))
  (return (struct) false))

(fn `GetDialogueLine`
  (returns (Line :type String))
  (bind (_currentdialogue_identifier _currentdialogue_dialogue) (break `/Game/Blueprints/Dialogue` (`self.CurrentDialogue`)))
  (bind _currentlineindex (`self.CurrentLineIndex`))
  (if (`KismetArrayLibrary.Array_IsValidIndex` _currentdialogue_dialogue _currentlineindex)
    (return (`|GetArrayItem` _currentdialogue_dialogue _currentlineindex))
    (else
      (return "LINE ERROR"))))

(fn `ProceedDialogue`
  (bind (_currentdialogue_identifier _currentdialogue_dialogue _currentdialogue_color _currentdialogue_allowplayermove) (break `/Game/Blueprints/Dialogue` (`self.CurrentDialogue`)))
  (bind (_currentdialogue_identifier_2 _currentdialogue_dialogue_2) (break `/Game/Blueprints/Dialogue` (`self.CurrentDialogue`)))
  (bind (_currentdialogue_identifier_3 _currentdialogue_dialogue_3 _currentdialogue_color_2) (break `/Game/Blueprints/Dialogue` (`self.CurrentDialogue`)))
  (if (`self.inDialogue`)
    (if (< (`self.CurrentLineIndex`) (- (`KismetArrayLibrary.Array_Length` _currentdialogue_dialogue_2) 1))
      (`/Engine/EditorBlueprintResources/StandardMacros.IncrementInt` (`self.CurrentLineIndex`)
        (:`  `
          (`/Game/Blueprints/Widget/WBP_Dialogue.SetText` (`self.DialogueWidget`) (`self.GetDialogueLine`) _currentdialogue_color_2)))
      (else
        (if (not _currentdialogue_allowplayermove)
          (bind _asbp_third_person_character (cast `/Game/ThirdPerson/Blueprints/BP_ThirdPersonCharacter` (`GameplayStatics.GetPlayerCharacter` 0)))
          (set `/Game/ThirdPerson/Blueprints/BP_ThirdPersonCharacter.canMove` true _asbp_third_person_character))
        (`self.ClearDialogue`)))))

(fn `TriggerDialogue`
  (params (Identifier :type String) (NumIdentifier :type Integer :default -1) (DialogueInstigator :type "Actor Object Reference") (CustomOffset :type "Vector Structure"))
  (returns (Success :type Boolean))
  (bind (_currentdialogue_identifier _currentdialogue_dialogue _currentdialogue_color) (break `/Game/Blueprints/Dialogue` (`self.CurrentDialogue`)))
  (bind (_out_dialogue _success) (`self.FindDialogueByID` (`local.Identifier`)))
  (set `self.inDialogue` false)
  (set `self.CurrentLineIndex` 0)
  (`|ExecutionSequence`
    (:`then_0`
      (if (`KismetStringLibrary.IsEmpty` Identifier)
        (if (!= NumIdentifier -1)
          (if (`KismetArrayLibrary.Array_IsValidIndex` (`self.Dialogues`) (`local.NumIdentifier`))
            (set `self.CurrentDialogue` (`|GetArrayItem` (`self.Dialogues`) (`local.NumIdentifier`)))
            (else
              (`KismetSystemLibrary.PrintString` "Invalid num identifier given" true true (struct :`R` 1.0 :`G` 0.029677 :`A` 1.0))
              (return false)))
          (else
            (return false)))
        (elif _success
          (set `self.CurrentDialogue` _out_dialogue)
          (else
            (`KismetSystemLibrary.PrintString` "Invalid identifier given" true true (struct :`R` 1.0 :`G` 0.029677 :`A` 1.0))
            (return false)))))
    (:`then_1`
      (`/Game/Blueprints/Widget/WBP_Dialogue.SetText` (`self.DialogueWidget`) (`self.GetDialogueLine`) _currentdialogue_color)
      (`self.K2_SetActorLocation` (+ (`self.K2_GetActorLocation` (`local.DialogueInstigator`)) (`KismetMathLibrary.SelectVector` (`self.PositionOffset`) (`local.CustomOffset`) (`KismetMathLibrary.Vector_IsZero` (`local.CustomOffset`)))))
      (set `self.inDialogue` true)
      (`self.DelaySetVisibility` true))))

(fn `UserConstructionScript`
  (`PrimitiveComponent.SetCastShadow` (`self.Widget`) false))