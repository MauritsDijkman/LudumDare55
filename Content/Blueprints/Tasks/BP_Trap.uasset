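; Rope-triggered trap that rolls a random effect at BeginPlay: poison, slow, or one of two damage amounts.
; When the player character overlaps the rope, it applies the effect, updates the current task and plays an activation sound.
; BP_FollowCapsule gets its own versions without the task update, though its slow is undone immediately, with no delay.
; Either overlap destroys the rope, making the trap single-use.
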(event `self.ReceiveBeginPlay`
  (set `self.TrapType` (`KismetArrayLibrary.Array_Random` (`|MakeArray` "NewEnumerator0" "NewEnumerator1" "NewEnumerator2" "NewEnumerator3" :!type "/Game/Blueprints/Tasks/TrapType Enum"))))

(event `self.Rope.OnComponentBeginOverlap`
  (params (OverlappedComponent :type "PrimitiveComponent Object Reference") (OtherActor :type "Actor Object Reference") (OtherComp :type "PrimitiveComponent Object Reference") (OtherBodyIndex :type Integer) (bFromSweep :type Boolean) (SweepResult :type "HitResult Structure (by ref)"))
  (bind _traptype (`self.TrapType`))
  (bind _asbp_third_person_character (cast `/Game/ThirdPerson/Blueprints/BP_ThirdPersonCharacter` OtherActor)
    (:`then`
      (`|ExecutionSequence`
        (:`then_0`
          (switch `/Game/Blueprints/Tasks/TrapType` _traptype
            (:`NewEnumerator0`
              (`/Game/ThirdPerson/Blueprints/BP_ThirdPersonCharacter.SetPoisoned` _asbp_third_person_character 5.0))
            (:`NewEnumerator1`
              (`/Game/ThirdPerson/Blueprints/BP_ThirdPersonCharacter.SetMaxWalkingSpeed` _asbp_third_person_character 0.3 true 10.0))
            (:`NewEnumerator2`
              (`/Game/Blueprints/BPI_Damagable.Damage` _asbp_third_person_character 25.0 (0.0 0.0 0.0)))
            (:`NewEnumerator3`
              (`/Game/Blueprints/BPI_Damagable.Damage` _asbp_third_person_character 50.0 (0.0 0.0 0.0))))
          (`/Game/ThirdPerson/Blueprints/BP_ThirdPersonCharacter.UpdateCurrentTask` _asbp_third_person_character 5)
          (`GameplayStatics.PlaySoundAtLocation` "/Game/Audio/SoundEffects/trap_activation.trap_activation" (`self.K2_GetActorLocation`) (struct) 1.0 1.0 0.0 null null null null))
        (:`then_1`
          (`ActorComponent.K2_DestroyComponent` (`self.Rope`) :!label _label))))
    (:`CastFailed`
      (bind _asbp_follow_capsule (cast `/Game/Blueprints/BP_FollowCapsule` OtherActor))
      (`|ExecutionSequence`
        (:`then_0`
          (switch `/Game/Blueprints/Tasks/TrapType` _traptype
            (:`NewEnumerator0`
              (set `/Game/Blueprints/BP_FollowCapsule.hasPoison` true _asbp_follow_capsule)
              (`KismetSystemLibrary.Delay` 5.0)
              (set `/Game/Blueprints/BP_FollowCapsule.hasPoison` false _asbp_follow_capsule))
            (:`NewEnumerator1`
              (bind _charactermovement (`Character.CharacterMovement` _asbp_follow_capsule))
              (bind _maxwalkspeed (`CharacterMovementComponent.MaxWalkSpeed` _charactermovement))
              (set `CharacterMovementComponent.MaxWalkSpeed` (* _maxwalkspeed 0.5) _charactermovement)
              (set `CharacterMovementComponent.MaxWalkSpeed` (* _maxwalkspeed 2.0) _charactermovement))
            (:`NewEnumerator2`
              (message `/Game/Blueprints/BPI_Damagable.Damage` _asbp_follow_capsule 25.0 (0.0 0.0 0.0)))
            (:`NewEnumerator3`
              (message `/Game/Blueprints/BPI_Damagable.Damage` _asbp_follow_capsule 50.0 (0.0 0.0 0.0))))
          (`GameplayStatics.PlaySoundAtLocation` "/Game/Audio/SoundEffects/trap_activation.trap_activation" (`self.K2_GetActorLocation`) (struct) 1.0 1.0 0.0 null null null null))
        (:`then_1`
          (goto _label))))))

(fn `UserConstructionScript`)