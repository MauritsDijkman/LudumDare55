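; BP_Bat is a bat actor that adds a visual hit effect to the damage handling of its parent class.
; BeginPlay creates dynamic material instances for the first two mesh slots.
; Damage triggers a timeline that drives the HitEffect scalar parameter on the first material only, then returns the parent's result.
; The second material instance is stored but not used in this Blueprint.
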(event `self.ReceiveBeginPlay`
  (bind _mesh (`self.Mesh`))
  (bind _mesh_2 (`self.Mesh`))
  (bind _returnvalue (`PrimitiveComponent.CreateDynamicMaterialInstance` _mesh_2 0 (`PrimitiveComponent.GetMaterial` _mesh 0) "None"))
  (set `self.Mat` _returnvalue)
  (bind _returnvalue_2 (`PrimitiveComponent.CreateDynamicMaterialInstance` _mesh_2 1 (`PrimitiveComponent.GetMaterial` _mesh 1) "None"))
  (set `self.Mat2` _returnvalue_2))

(event `HitEffect`
  (bind _mat (`self.Mat`)
    (:`then`
      (bind (_direction _curve) (`Timeline|Timeline` :!via `PlayFromStart`)
        (:`Update`
          (`MaterialInstanceDynamic.SetScalarParameterValue` _mat "HitEffect" _curve))))
    (:`else`)))

(fn `Damage`
  (params (Amt :type "Float (double-precision)") (Normal :type "Vector Structure"))
  (returns (Dead :type Boolean))
  (`self.HitEffect`)
  (bind _dead (`parent.Damage` Amt Normal))
  (return _dead))

(fn `UserConstructionScript`
  (`parent.UserConstructionScript`))