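; BP_FixedCamera is a camera actor that smoothly follows the first player's character within set horizontal bounds.
; BeginPlay caches the character, then Tick adds an offset to its location and clamps X and Y to the min/max limits.
; The actor lerps toward that point by delta time times follow speed, while its height stays at the offset's absolute Z, ignoring the character's height.
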(event `self.ReceiveBeginPlay`
  ;[1 1 1] Event - BeginPlay
  (set `self.Player` (`GameplayStatics.GetPlayerCharacter` 0)))

(event `self.ReceiveTick`
  (params (DeltaSeconds :type "Float (single-precision)"))
  (bind (_offset_x _offset_y _offset_z) (`KismetMathLibrary.BreakVector` (`self.Offset`)))
  (bind (_returnvalue_x _returnvalue_y _returnvalue_z) (`KismetMathLibrary.BreakVector` (+ (`self.K2_GetActorLocation` (`self.Player`)) (`self.Offset`))))
  (bind (_returnvalue_x_2 _returnvalue_y_2) (`KismetMathLibrary.BreakVector` (`KismetMathLibrary.VLerp` (`self.K2_GetActorLocation`) (`KismetMathLibrary.MakeVector` (`KismetMathLibrary.FClamp` _returnvalue_x (`self.MinX`) (`self.MaxX`)) (`KismetMathLibrary.FClamp` _returnvalue_y (`self.MinY`) (`self.MaxY`)) _returnvalue_z) (* DeltaSeconds (`self.FollowSpeed`)))))
  ;[1 1 1] Event - Tick
  (`self.K2_SetActorLocationAndRotation` (`KismetMathLibrary.MakeVector` _returnvalue_x_2 _returnvalue_y_2 _offset_z)))

(fn `UserConstructionScript`)