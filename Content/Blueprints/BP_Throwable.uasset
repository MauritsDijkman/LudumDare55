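; BP_Throwable is a projectile that damages what it hits, launched by an Init function that sets the ProjectileMovement velocity and makes rotation follow it.
; Sphere overlaps with actors of a different class than the Instigator send DamageMessage through BPI_Damagable if implemented.
; Those damaging overlaps, and any blocking Sphere hit, add a Niagara component, set User.Hit, destroy the Sphere and set a short lifespan.
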(event `self.Sphere.OnComponentBeginOverlap`
  (params (OverlappedComponent :type "PrimitiveComponent Object Reference") (OtherActor :type "Actor Object Reference") (OtherComp :type "PrimitiveComponent Object Reference") (OtherBodyIndex :type Integer) (bFromSweep :type Boolean) (SweepResult :type "HitResult Structure (by ref)"))
  ;[1 1 1] Pawn
  (if (!= (`GameplayStatics.GetObjectClass` OtherActor) (`GameplayStatics.GetObjectClass` (`self.Instigator`)))
    (if (`KismetSystemLibrary.DoesImplementInterface` OtherActor "/Game/Blueprints/BPI_Damagable.BPI_Damagable_C")
      (message `/Game/Blueprints/BPI_Damagable.Damage` OtherActor (`self.Damage`) (`KismetMathLibrary.Normal` (- (`self.K2_GetActorLocation`) (`self.K2_GetActorLocation`))))
      ;[1 1 1] Environment
      (`AddComponent|NODE_AddNiagaraComponent-0` :!label _label)
      (`NiagaraComponent.SetVariableBool` (`self.Niagara`) "User.Hit" true)
      (`ActorComponent.K2_DestroyComponent` (`self.Sphere`))
      (`self.SetLifeSpan` 2.0))))

(event `self.Sphere.OnComponentHit`
  (params (HitComponent :type "PrimitiveComponent Object Reference") (OtherActor :type "Actor Object Reference") (OtherComp :type "PrimitiveComponent Object Reference") (NormalImpulse :type "Vector Structure") (Hit :type "HitResult Structure (by ref)"))
  ;[1 1 1] Environment
  (goto _label))

(fn `Init`
  (params (LaunchVelociy :type "Vector Structure"))
  (bind _projectilemovement (`self.ProjectileMovement`))
  (`KismetSystemLibrary.PrintString` "BP_Throwable Init")
  (set `MovementComponent.Velocity` LaunchVelociy _projectilemovement)
  (set `ProjectileMovementComponent.bRotationFollowsVelocity` true _projectilemovement))

(fn `UserConstructionScript`)