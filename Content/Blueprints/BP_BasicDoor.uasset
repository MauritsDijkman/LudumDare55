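; BP_BasicDoor is an interactable door that moves the interactor between two rooms, showing the destination and hiding the room left behind.
; A dot product against the door's forward vector picks the direction and entry point.
; The far room is spawned lazily as a BP_BasicRoom, offset by its size along the door's backward axis, then generated.
; The door destroys itself when its bound room is destroyed.
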(event `/Game/Blueprints/I_Interactable.Interact`
  (params (Interactor :type "Character Object Reference"))
  (if (`self.Check Door Dir` Interactor)
    (`self.SetActorHiddenInGame` (`self.Room`) false)
    (`self.SetActorHiddenInGame` (`self.Room2`) true)
    (else
      (`self.SetActorHiddenInGame` (`self.Room`) true)
      (bind _room2 (`self.Room2`)
        (:`then`
          (`self.SetActorHiddenInGame` _room2 false))
        (:`else`
          (`self.SpawnNewRoom`)))))
  (`self.MoveInteractor` Interactor))

(event `BindRoom`
  (params (Room :type "/Game/Blueprints/BP_BasicRoom Object Reference"))
  (bind _output_get (set `self.Room` Room))
  (add `self.OnDestroyed` _output_get (delegate `OnRoomDestroyed`)))

(event `OnRoomDestroyed` :!signature `self.OnDestroyed`
  (params (DestroyedActor :type "Actor Object Reference"))
  (`self.K2_DestroyActor`))

(fn `Check Door Dir`
  (params (Interactor :type "Actor Object Reference"))
  (returns (isOldRoom :type Boolean))
  (return (< (`KismetMathLibrary.Dot_VectorVector` (- (`self.K2_GetActorLocation` Interactor) (`self.K2_GetActorLocation`)) (`self.GetActorForwardVector`)) 0.0)))

(fn `MoveInteractor`
  (params (Interactor :type "Actor Object Reference"))
  (`self.K2_SetActorLocation` Interactor (`SceneComponent.K2_GetComponentLocation` (select `bool` (`self.Check Door Dir` Interactor) :`false` (`self.Player Entry Point`) :`true` (`self.Player Entry Back`))) false false))

(fn `SpawnNewRoom`
  (`KismetSystemLibrary.PrintString` "Spawned New Room")
  (bind _returnvalue (`|SpawnActorFromClass` "/Game/Blueprints/BP_BasicRoom.BP_BasicRoom_C" (`KismetMathLibrary.MakeTransform` (`self.K2_GetActorLocation` (`self.Room`))) "Undefined" "MultiplyWithRoot" null null))
  (set `self.Room2` _returnvalue)
  (bind _roomsize_x (`KismetMathLibrary.BreakVector2D` (`/Game/Blueprints/BP_BasicRoom.RoomSize` _returnvalue)))
  (`self.K2_AddActorWorldOffset` _returnvalue (* (* (`self.GetActorForwardVector`) -1) _roomsize_x) false true)
  (`/Game/Blueprints/BP_BasicRoom.Generate` (`self.Room2`)))

(fn `UserConstructionScript`)