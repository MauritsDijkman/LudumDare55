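; BP_ExpOrb is an experience pickup that homes in on the player character.
; Each tick it lerps toward the player's location with delta time as alpha, so it moves faster when farther away.
; Overlapping its Sphere with BP_ThirdPersonCharacter grants a fixed amount of experience, plays a sound at a randomized pitch, and destroys the orb.
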(event `self.ReceiveBeginPlay`
  (set `self.Player` (`GameplayStatics.GetPlayerCharacter` 0)))

(event `self.ReceiveTick`
  (params (DeltaSeconds :type "Float (single-precision)"))
  (`self.K2_SetActorLocation` (`KismetMathLibrary.VLerp` (`self.K2_GetActorLocation`) (`self.K2_GetActorLocation` (`self.Player`)) DeltaSeconds)))

(event `self.Sphere.OnComponentBeginOverlap`
  (params (OverlappedComponent :type "PrimitiveComponent Object Reference") (OtherActor :type "Actor Object Reference") (OtherComp :type "PrimitiveComponent Object Reference") (OtherBodyIndex :type Integer) (bFromSweep :type Boolean) (SweepResult :type "HitResult Structure (by ref)"))
  (bind _asbp_third_person_character (cast `/Game/ThirdPerson/Blueprints/BP_ThirdPersonCharacter` OtherActor))
  (`/Game/ThirdPerson/Blueprints/BP_ThirdPersonCharacter.AddExp` _asbp_third_person_character 4)
  (`GameplayStatics.PlaySoundAtLocation` "/Game/Audio/SoundEffects/exp_orb.exp_orb" (`self.K2_GetActorLocation`) (struct) 1.0 (/ (`KismetMathLibrary.RandomIntegerInRange` 8 12) 10.0) 0.0 null null null null)
  (`self.K2_DestroyActor`))

(fn `UserConstructionScript`)