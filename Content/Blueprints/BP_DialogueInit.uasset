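; BP_DialogueInit is a placeable trigger that starts a dialogue through the level's BP_DialogueManager.
; It finds the manager on BeginPlay, then fires its DialogueIdentifier when BP_ThirdPersonCharacter overlaps its sphere or InitDialogue is called, passing itself as instigator with a raised offset.
; An optional UseOnce flag limits it to a single trigger.
; The construction script sizes the sphere from the Size variable.
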(event `self.ReceiveBeginPlay`
  (bind _returnvalue (`GameplayStatics.GetActorOfClass` "/Game/Blueprints/BP_DialogueManager.BP_DialogueManager_C"))
  (set `self.DManager` _returnvalue))

(event `self.Sphere.OnComponentBeginOverlap`
  (params (OverlappedComponent :type "PrimitiveComponent Object Reference") (OtherActor :type "Actor Object Reference") (OtherComp :type "PrimitiveComponent Object Reference") (OtherBodyIndex :type Integer) (bFromSweep :type Boolean) (SweepResult :type "HitResult Structure (by ref)"))
  (cast `/Game/ThirdPerson/Blueprints/BP_ThirdPersonCharacter` OtherActor)
  (if (`self.useOnce`) :!label _label
    (if (not (`self.used`))
      (set `self.used` true)
      (`/Game/Blueprints/BP_DialogueManager.TriggerDialogue` (`self.DManager`) (`self.DialogueIdentifier`) -1 self (0.0 0.0 200.0) :!label _label_2))
    (else
      (goto _label_2))))

(event `InitDialogue`
  (goto _label))

(fn `UserConstructionScript`
  (`SphereComponent.SetSphereRadius` (`self.Sphere`) (`self.size`) true))