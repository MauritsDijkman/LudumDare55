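; Final boss mage that faces the player and fights with projectiles, a shield and teleports; starting the fight switches music and shows boss health.
; A randomized Tick timer picks among six throwable types, a temporary damage-reduction shield, or a weighted teleport to room-relative points.
; Orb color, Niagara and usually sound telegraph each action.
; Damage scales by resistance and updates the player's UI; death unlocks room doors and loads the credits.
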(event `startFight`
  (bind _returnvalue (`GameplayStatics.GetActorOfClass` "/Game/Audio/Blueprints/BP_MusicHandler.BP_MusicHandler_C"))
  (`/Engine/EditorBlueprintResources/StandardMacros.IsValid` _returnvalue
    (:`Is Valid`
      (`/Game/Audio/Blueprints/BP_MusicHandler.HandleMusic` _returnvalue "NewEnumerator4")
      (`self.UpdateHbar`)
      (set `self.timeBeforeNextAttack` 2.0))))

(event `self.ReceiveBeginPlay`
  (set `self.health` (`self.maxhealth`))
  (bind _returnvalue (`PrimitiveComponent.CreateDynamicMaterialInstance` (`self.StaticMesh`) 1 "/Game/Blueprints/Mage/MageBall.MageBall" "None"))
  (set `self.Ball` _returnvalue)
  (bind _asbp_third_person_character (cast `/Game/ThirdPerson/Blueprints/BP_ThirdPersonCharacter` (`GameplayStatics.GetPlayerCharacter` 0)))
  (set `self.Player` _asbp_third_person_character)
  (bind _returnvalue_2 (`PrimitiveComponent.CreateDynamicMaterialInstance` (`self.Shield`) 0 "/Game/Materials/Shield/M_Shield.M_Shield" "None"))
  (set `self.ShieldMat` _returnvalue_2)
  (if (`self.autoStartFight`)
    (`self.startFight`)))

(event `self.ReceiveTick`
  (params (DeltaSeconds :type "Float (single-precision)"))
  (`|ExecutionSequence`
    (:`then_0`
      (bind _time_for_attack (`self.UpdateTimer` DeltaSeconds))
      (if _time_for_attack
        (switch `int` (`KismetMathLibrary.RandomInteger` 10)
          (:`0`
            (`self.SetBallColor` (struct :`R` 1.0 :`G` 0.178082 :`A` 1.0))
            (`KismetSystemLibrary.Delay` 0.5)
            (`self.SpawnThrowable` "/Game/Blueprints/Throwables/BP_Throwable.BP_Throwable_C" 2000.0 20.0)
            (`self.SetBallColor` (struct :`R` 1.0 :`G` 1.0 :`B` 1.0 :`A` 1.0) false :!label _label))
          (:`1`
            (`self.SetBallColor` (struct :`R` 0.335497 :`G` 0.338542 :`B` 0.311685 :`A` 1.0))
            (`KismetSystemLibrary.Delay` 0.5)
            (`self.SpawnThrowable` "/Game/Blueprints/Mage/Attacks/BP_SlowingAttack.BP_SlowingAttack_C" 1000.0 5.0)
            (goto _label))
          (:`2`
            (`self.SetBallColor` (struct :`G` 0.463542 :`B` 0.094044 :`A` 1.0))
            (`KismetSystemLibrary.Delay` 0.5)
            (`self.SpawnThrowable` "/Game/Blueprints/Mage/Attacks/BP_PoisonAttack.BP_PoisonAttack_C" 1500.0 5.0)
            (goto _label))
          (:`3`
            (`self.SetBallColor` (struct :`G` 0.280793 :`B` 1.0 :`A` 1.0))
            (`KismetSystemLibrary.Delay` 0.5)
            (`self.SpawnThrowable` "/Game/Blueprints/Mage/Attacks/BP_HomingAttack.BP_HomingAttack_C" 5.0 30.0)
            (goto _label))
          (:`4`
            (`self.SetBallColor` (struct :`R` 1.0 :`G` 0.645608 :`A` 1.0))
            (`KismetSystemLibrary.Delay` 0.5)
            (`self.SpawnThrowable` "/Game/Blueprints/Mage/Attacks/BP_KnockbackBolt.BP_KnockbackBolt_C" 2000.0 15.0)
            (goto _label))
          (:`5`
            (`self.SetBallColor` (struct :`A` 1.0))
            (`KismetSystemLibrary.Delay` 0.5)
            (`self.SpawnThrowable` "/Game/Blueprints/Mage/Attacks/BP_ExplosionAttack.BP_ExplosionAttack_C" 300.0)
            (goto _label))
          (:`6`
            (`self.SetBallColor` (struct :`R` 0.207907 :`B` 1.0 :`A` 1.0))
            (`KismetSystemLibrary.Delay` 0.5)
            (`MaterialInstanceDynamic.SetScalarParameterValue` (`self.ShieldMat`) "HitEffect" 1.0)
            (set `self.resistence` 0.25)
            (`|ExecutionSequence`
              (:`then_0`
                (goto _label))
              (:`then_1`
                (`KismetSystemLibrary.RetriggerableDelay` 5.0)
                (`MaterialInstanceDynamic.SetScalarParameterValue` (`self.ShieldMat`) "HitEffect" 0.0)
                (set `self.resistence` 0.5))))
          (:`7`
            (set `self.TargetPosition` (+ (`KismetArrayLibrary.Array_Random` (`self.TeleportPositions`)) (`self.RoomCenter`)) :!label _label_2)
            (if (!= (`self.TargetPosition`) (`self.K2_GetActorLocation`) :`ErrorTolerance` 100.0)
              (`self.SetBallColor` (struct :`R` 1.0 :`B` 0.924093 :`A` 1.0))
              (`NiagaraComponent.SetVariableBool` (`self.NS_TeleportSmoke`) "User.Spawn" true)
              (`|ExecutionSequence`
                (:`then_0`
                  (`KismetSystemLibrary.Delay` 1.0)
                  (`NiagaraComponent.SetVariableBool` (`self.NS_TeleportSmoke`) "User.Spawn" false)
                  (`self.K2_SetActorLocation` (`self.TargetPosition`) false true)
                  (`AddComponent|NODE_AddNiagaraComponent-0`))
                (:`then_1`
                  (goto _label)))))
          (:`8`
            (goto _label_2))
          (:`9`
            (goto _label_2)))))
    (:`then_1`
      (`self.Look At Player`))))

(event `Charge`
  (`NiagaraComponent.SetVariableBool` (`self.Niagara`) "User.Spawn" true)
  (`KismetSystemLibrary.Delay` 0.2)
  (`NiagaraComponent.SetVariableBool` (`self.Niagara`) "User.Spawn" false))

(fn `Damage`
  (params (Amt :type "Float (double-precision)") (Normal :type "Vector Structure"))
  (returns (Dead :type Boolean))
  (bind _player (`self.Player`))
  (bind _output_get (set `self.health` (- (`self.health`) (* Amt (`self.resistence`) 1.5))))
  (`self.UpdateHbar`)
  (if (< _output_get 0.0)
    (`|ExecutionSequence`
      (:`then_0`
        (set `/Game/ThirdPerson/Blueprints/BP_ThirdPersonCharacter.defeatedBoss` true _player)
        (`/Game/ThirdPerson/Blueprints/BP_ThirdPersonCharacter.Reload Level After Seconds` _player "L_CreditsMenu" 3.0 true))
      (:`then_1`
        (bind _returnvalue (`GameplayStatics.GetActorOfClass` "/Game/Blueprints/Mage/BP_BossRoom.BP_BossRoom_C"))
        (`/Engine/EditorBlueprintResources/StandardMacros.IsValid` _returnvalue
          (:`Is Valid`
            (`/Game/Blueprints/Mage/BP_BossRoom.SetDoorsInteractable` _returnvalue true))))
      (:`then_2`
        (`self.SetLifeSpan` 0.5)
        (return true)))
    (else
      (return false))))

(fn `Look At Player`
  (bind (_returnvalue_x _returnvalue_y) (`KismetMathLibrary.BreakVector` (- (`self.K2_GetActorLocation` (`self.Player`)) (`self.K2_GetActorLocation`))))
  (`SceneComponent.K2_SetWorldRotation` (`self.StaticMesh`) (`KismetMathLibrary.ComposeRotators` (`KismetMathLibrary.FindLookAtRotation` (0.0 0.0 0.0) (`KismetMathLibrary.MakeVector` _returnvalue_x _returnvalue_y)) (`self.RotationOffset`)) false false))

(fn `SetBallColor`
  (params (Value :type "LinearColor Structure") (show :type Boolean :default true))
  (bind _ball (`self.Ball`)
    (:`then`
      (`MaterialInstanceDynamic.SetVectorParameterValue` _ball "Color" Value)
      (`NiagaraComponent.SetVariableLinearColor` (`self.Niagara`) "User.Color" Value)
      (if show
        (`self.Charge`)
        (`GameplayStatics.PlaySoundAtLocation` "/Game/Audio/SoundEffects/magicgather.magicgather" (`SceneComponent.K2_GetComponentLocation` (`self.ShootPoint`)) (struct) 1.0 1.0 0.0 null null null null)))
    (:`else`)))

(fn `SpawnThrowable`
  (params (Class :type "/Game/Blueprints/Throwables/BP_Throwable Class Reference") (Vel :type "Float (double-precision)") (Damage :type "Float (double-precision)"))
  (bind (_returnvalue_x _returnvalue_y _returnvalue_z) (`KismetMathLibrary.BreakVector` (* (`KismetMathLibrary.Normal` (- (`self.K2_GetActorLocation` (`self.Player`)) (`SceneComponent.K2_GetComponentLocation` (`self.ShootPoint`)))) (`local.Vel`))))
  (bind _returnvalue (`|SpawnActorFromClass` Class (`KismetMathLibrary.Conv_VectorToTransform` (`SceneComponent.K2_GetComponentLocation` (`self.ShootPoint`))) "Undefined" "MultiplyWithRoot" self self))
  (set `/Game/Blueprints/Throwables/BP_Throwable.Damage` (`local.Damage`) _returnvalue)
  (`/Game/Blueprints/Throwables/BP_Throwable.Init` _returnvalue (`KismetMathLibrary.MakeVector` _returnvalue_x _returnvalue_y _returnvalue_z)))

(fn `UpdateHbar`
  (bind _player (`self.Player`)
    (:`then`
      (bind _ui (`/Game/ThirdPerson/Blueprints/BP_ThirdPersonCharacter.UI` _player)
        (:`then`
          (`/Game/Blueprints/Widgets/BP_MainWidget.SetMageHealth` _ui (`self.health`) (`self.maxhealth`)))
        (:`else`)))
    (:`else`)))

(fn `UpdateTimer`
  (params (DTime :type "Float (double-precision)"))
  (returns (`Time for attack` :type Boolean))
  (bind _output_get (set `self.timeBeforeNextAttack` (- (`self.timeBeforeNextAttack`) DTime)))
  (if (<= _output_get 0.0)
    (set `self.timeBeforeNextAttack` (`KismetMathLibrary.RandomFloatInRange` 0.5 1.5))
    (return true)
    (else
      (return false))))

(fn `UserConstructionScript`)