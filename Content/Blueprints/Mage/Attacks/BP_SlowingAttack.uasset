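; BP_SlowingAttack is a mage attack that slows the character it hits.
; It overrides OnHit, calling the parent with zero explosion size and black color instead of forwarding those inputs, then casts the target to BP_ThirdPersonCharacter.
; On that character it sets a ten-second SlowedTimeLeft, halves walk speed from OriginalMaxSpeed so hits don't stack, and flags IsSlowed; restoring speed is not handled here.
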(event `self.ReceiveBeginPlay`
  (`parent.ReceiveBeginPlay`))

(fn `OnHit`
  (params (Target :type "Character Object Reference") (ExplosionSIze :type "Float (double-precision)") (ExplosionColor :type "LinearColor Structure"))
  (`parent.OnHit` Target 0.0 (struct))
  (bind _asbp_third_person_character (cast `/Game/ThirdPerson/Blueprints/BP_ThirdPersonCharacter` Target))
  (set `/Game/ThirdPerson/Blueprints/BP_ThirdPersonCharacter.SlowedTimeLeft` 10.0 _asbp_third_person_character)
  (set `CharacterMovementComponent.MaxWalkSpeed` (* (`/Game/ThirdPerson/Blueprints/BP_ThirdPersonCharacter.OriginalMaxSpeed` _asbp_third_person_character) 0.5) (`Character.CharacterMovement` _asbp_third_person_character))
  (set `/Game/ThirdPerson/Blueprints/BP_ThirdPersonCharacter.IsSlowed` true _asbp_third_person_character))

(fn `UserConstructionScript`
  (`parent.UserConstructionScript`))