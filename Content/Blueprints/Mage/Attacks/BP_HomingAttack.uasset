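; BP_HomingAttack is a Mage attack projectile that homes in on the player character.
; On BeginPlay it casts player 0 to BP_ThirdPersonCharacter and sets that character's Center component as the ProjectileMovement homing target.
; It overrides the parent's Init with an empty body, leaving the parent call disconnected, so the launch velocity argument is unused.
; OnExplode runs the parent logic, then hides Sphere1.
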(event `self.ReceiveBeginPlay`
  (bind _asbp_third_person_character (cast `/Game/ThirdPerson/Blueprints/BP_ThirdPersonCharacter` (`GameplayStatics.GetPlayerCharacter` 0)))
  (set `ProjectileMovementComponent.HomingTargetComponent` (`/Game/ThirdPerson/Blueprints/BP_ThirdPersonCharacter.Center` _asbp_third_person_character) (`self.ProjectileMovement`)))

(fn `Init`
  (params (LaunchVelociy :type "Vector Structure")))

(fn `OnExplode`
  (`parent.OnExplode`)
  (`SceneComponent.SetVisibility` (`self.Sphere1`) false false))

(fn `UserConstructionScript`
  (`parent.UserConstructionScript`))