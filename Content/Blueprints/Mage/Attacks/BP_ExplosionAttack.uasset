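; BP_ExplosionAttack is a mage attack that damages a character caught in its blast.
; It overrides OnExplode, calling the parent logic and then querying Sphere1 for overlapping BP_ThirdPersonCharacter actors.
; Only the first character found receives a fixed DamageMessage with a zero normal.
; The Niagara component is added only when such a character is hit.
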(event `self.ReceiveBeginPlay`
  (`parent.ReceiveBeginPlay`))

(fn `OnExplode`
  (bind _overlappingactors (`PrimitiveComponent.GetOverlappingActors` (`self.Sphere1`) "/Game/ThirdPerson/Blueprints/BP_ThirdPersonCharacter.BP_ThirdPersonCharacter_C"))
  (`parent.OnExplode`)
  (if (`KismetArrayLibrary.Array_IsNotEmpty` _overlappingactors)
    (message `/Game/Blueprints/BPI_Damagable.Damage` (`|GetArrayItem` _overlappingactors) 50.0 (0.0 0.0 0.0))
    (`AddComponent|NODE_AddNiagaraComponent-0`)))

(fn `UserConstructionScript`
  (`parent.UserConstructionScript`))