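; Enemy spawn volume that populates its parent BP_BasicRoom with one to five random enemies shortly after play begins.
; Construction sizes the box from Bounds, and SpawnEnemies places random EnemyClasses picks at random points inside it at a fixed height.
; Each spawned BP_FollowCapsule is bound to the room and a death event.
; EnemiesLeft tracks survivors, switching BP_MusicHandler's music state after spawning and again when all are dead.
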(event `self.ReceiveBeginPlay`
  (`KismetSystemLibrary.Delay` 0.2)
  (`self.SpawnEnemies` (`KismetMathLibrary.RandomIntegerInRange` 1 5))
  (if (> (`self.EnemiesLeft`) 0)
    (bind _returnvalue (`GameplayStatics.GetActorOfClass` "/Game/Audio/Blueprints/BP_MusicHandler.BP_MusicHandler_C"))
    (`/Engine/EditorBlueprintResources/StandardMacros.IsValid` _returnvalue
      (:`Is Valid`
        (`/Game/Audio/Blueprints/BP_MusicHandler.HandleMusic` _returnvalue "NewEnumerator3")))))

(event `OnEnemyDeath`
  (bind _result (`/Engine/EditorBlueprintResources/StandardMacros.DecrementInt` (`self.EnemiesLeft`))
    (:`  `
      (if (<= _result 0)
        (bind _returnvalue (`GameplayStatics.GetActorOfClass` "/Game/Audio/Blueprints/BP_MusicHandler.BP_MusicHandler_C"))
        (`/Engine/EditorBlueprintResources/StandardMacros.IsValid` _returnvalue
          (:`Is Valid`
            (`/Game/Audio/Blueprints/BP_MusicHandler.HandleMusic` _returnvalue "NewEnumerator2")))))))

(fn `SpawnEnemies`
  (params (Amt :type Integer))
  (bind (_returnvalue_x _returnvalue_y) (`KismetMathLibrary.BreakVector` (+ (`self.K2_GetActorLocation`) (`KismetMathLibrary.RandomPointInBoundingBox` (0.0 0.0 0.0) (`.BoxExtent` (`KismetSystemLibrary.GetComponentBounds` (`self.Box`)))))))
  (set `self.EnemiesLeft` Amt)
  (for _ (range 1 (+ Amt 1))
    (bind _asbp_basic_room (cast `/Game/Blueprints/BP_BasicRoom` (`self.GetParentActor`)))
    (set `self.Room` _asbp_basic_room)
    (bind _returnvalue (`|SpawnActorFromClass` (`KismetArrayLibrary.Array_Random` (`self.EnemyClasses`)) (`KismetMathLibrary.MakeTransform` (`KismetMathLibrary.MakeVector` _returnvalue_x _returnvalue_y 88.0)) "Undefined" "MultiplyWithRoot" null null))
    (bind _asbp_follow_capsule (cast `/Game/Blueprints/BP_FollowCapsule` _returnvalue))
    (`/Engine/EditorBlueprintResources/StandardMacros.IsValid` _asbp_follow_capsule
      (:`Is Valid`
        (`/Game/Blueprints/BP_FollowCapsule.Bind Room` _asbp_follow_capsule (`self.Room`))
        (add `/Game/Blueprints/BP_FollowCapsule.OnDeath` _asbp_follow_capsule (`|CreateDelegate` :!event `OnEnemyDeath`))))))

(fn `UserConstructionScript`
  (`BoxComponent.SetBoxExtent` (`self.Box`) (/ (`self.Bounds`) 2) false))