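; BP_FollowCapsule is a room-bound enemy that chases the player, with optional melee and ranged attacks.
; An AI move loop melees on arrival, while a randomized looping timer launches BP_Throwable projectiles toward the player.
; The room's visibility updates drive Sleep, which hides the mesh and health bar and pauses the ranged timer.
; Damage applies knockback and blood splatter, updates the health bar, and fires OnDeath before destroying the actor.
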(event `Bind Room`
  (params (SpawnedRoom :type "/Game/Blueprints/BP_BasicRoom Object Reference"))
  (bind _widget (`self.Widget`))
  (`|ExecutionSequence`
    (:`then_0`
      (bind _output_get (set `self.SpawnedRoom` SpawnedRoom))
      (add `/Game/Blueprints/BP_BasicRoom.OnRoomVisibilityUpdate` _output_get (delegate `OnRoomVisibilityUpdate_Event`))
      (set `self.Player` (`GameplayStatics.GetPlayerCharacter` 0))
      (`self.Follow Player`)
      (if (`self.canRange`)
        (bind _returnvalue (`KismetSystemLibrary.K2_SetTimerDelegate` (delegate `Range`) (`KismetMathLibrary.RandomFloatInRange` 2.0 4.0) true (`KismetMathLibrary.RandomFloatInRange` 0.0 1.0)))
        (set `self.timer` _returnvalue)))
    (:`then_1`
      (bind _aswbp_healthbar (cast `/Game/Blueprints/Widgets/WBP_Healthbar` (`WidgetComponent.GetWidget` _widget))
        (:`then`
          (set `self.Healthbar` _aswbp_healthbar))
        (:`CastFailed`
          _))
      (set `self.health` (`self.maxHealth`))
      (`PrimitiveComponent.SetCastShadow` _widget false))))

(event `OnRoomVisibilityUpdate_Event`
  (params (Visible :type Boolean))
  (`self.Sleep` (not Visible)))

(event `Range`
  (bind (_returnvalue_x _returnvalue_y) (`KismetMathLibrary.BreakVector` (* (`KismetMathLibrary.Normal` (- (`self.K2_GetActorLocation` (`self.Player`)) (`self.K2_GetActorLocation`))) (`self.Throwable Launch Velocity`))))
  (`|AIMoveTo` null (`self.K2_GetActorLocation`) null
    (:`then`
      (bind _returnvalue (`|SpawnActorFromClass` "/Game/Blueprints/BP_Throwable.BP_Throwable_C" (`KismetMathLibrary.Conv_VectorToTransform` (`self.K2_GetActorLocation`)) "Undefined" "MultiplyWithRoot" self self))
      (set `/Game/Blueprints/BP_Throwable.Damage` (`self.Projectile Dmg`) _returnvalue)
      (`/Game/Blueprints/BP_Throwable.Init` _returnvalue (`KismetMathLibrary.MakeVector` _returnvalue_x _returnvalue_y 100.0)))))

(event `Follow Player`
  (bind _player (`self.Player`)
    (:`then`
      _)
    (:`else`
      (set `self.Player` (`GameplayStatics.GetPlayerCharacter` 0))))
  (`|AIMoveTo` self (0.0 0.0 0.0) _player
    (:`OnSuccess`
      (`self.MeleeAttack`)
      (if (not (`SceneComponent.bHiddenInGame` (`self.Mesh`)))
        (`self.Follow Player`)))))

(event `MeleeAttack`
  (bind _player (`self.Player`))
  (if (`self.canMelee`)
    (if (not (`self.isAttacking`))
      (set `self.isAttacking` true)
      (message `/Game/Blueprints/BPI_Damagable.Damage` _player (`self.meleeStrength`) (`KismetMathLibrary.Normal` (- (`self.K2_GetActorLocation` _player) (`self.K2_GetActorLocation`))))
      (`KismetSystemLibrary.Delay` 1.0)
      (set `self.isAttacking` false))))

(fn `Damage`
  (params (Amt :type "Float (double-precision)") (Normal :type "Vector Structure"))
  (returns (Dead :type Boolean))
  (`self.K2_AddActorWorldOffset` (* Normal 50.0))
  (`|SpawnActorFromClass` "/Game/Blueprints/BP_Bloodsplatter.BP_Bloodsplatter_C" (`KismetMathLibrary.MakeTransform` (`self.K2_GetActorLocation`) (`KismetMathLibrary.FindLookAtRotation` (0.0 0.0 0.0) Normal)) "Undefined" "MultiplyWithRoot" null null)
  (bind _output_get (set `self.health` (- (`self.health`) Amt)))
  (`/Game/Blueprints/Widgets/WBP_Healthbar.SetValue` (`self.Healthbar`) (/ _output_get (`self.maxHealth`)))
  (if (<= _output_get 0.0)
    (`self.OnDeath`)
    (`self.K2_DestroyActor`)
    (return true)))

(fn `Sleep`
  (params (Sleep :type Boolean :default true))
  (bind _timer (`self.timer`))
  (`|ExecutionSequence`
    (:`then_0`
      (`SceneComponent.SetHiddenInGame` (`self.Widget`) Sleep false)
      (`SceneComponent.SetHiddenInGame` (`self.Mesh`) Sleep true)
      (if Sleep
        (`KismetSystemLibrary.PrintString` "Sleeping..")
        (else
          (`self.Follow Player`))))
    (:`then_1`
      (if Sleep
        (`KismetSystemLibrary.K2_PauseTimerHandle` _timer)
        (else
          (`KismetSystemLibrary.K2_UnPauseTimerHandle` _timer))))))

(fn `UserConstructionScript`)