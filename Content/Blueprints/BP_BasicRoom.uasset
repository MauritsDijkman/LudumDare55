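; BP_BasicRoom is a modular room for procedural level generation that creates and links its own doors.
; Generate clears attached doors, links overlapping doors from other rooms as their second room, then removes those walls from the spawn candidates.
; Remaining door volumes may randomly spawn an attached door at a random point, skipping room overlaps and discarding doors that overlap others.
; SetRoomVisibility toggles visibility and collision for the room and its doors.
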(event `self.ReceiveBeginPlay`
  (for _array_element (`self.GetAttachedActors` true)
    (bind _asbp_basic_door (cast `/Game/Blueprints/BP_BasicDoor` _array_element))
    (`KismetArrayLibrary.Array_Add` (`self.Doors`) _asbp_basic_door)
    (`KismetSystemLibrary.PrintString` (`KismetSystemLibrary.GetDisplayName` _asbp_basic_door))))

(event `Generate`
  (`self.DestroyExistingDoors`)
  (`self.FillArray`)
  (`self.BindDoors`)
  (`self.SpawnDoors`))

(fn `BindDoors`
  (for _array_element (`PrimitiveComponent.GetOverlappingActors` (`self.RoomCollider`) "/Game/Blueprints/BP_BasicDoor.BP_BasicDoor_C")
    (bind _asbp_basic_door (cast `/Game/Blueprints/BP_BasicDoor` _array_element))
    (`KismetArrayLibrary.Array_Add` (`self.Doors`) _asbp_basic_door)
    (if (!= (`/Game/Blueprints/BP_BasicDoor.Room` _asbp_basic_door) self)
      (set `/Game/Blueprints/BP_BasicDoor.Room2` self _asbp_basic_door)
      (for _array_element_2 (`self.DoorWalls`)
        (if (`PrimitiveComponent.IsOverlappingActor` _array_element_2 _asbp_basic_door)
          (`KismetArrayLibrary.Array_RemoveItem` (`self.DoorWalls`) _array_element_2))))))

(fn `DestroyExistingDoors`
  (for _array_element (`self.GetAttachedActors` true)
    (bind _asbp_basic_door (cast `/Game/Blueprints/BP_BasicDoor` _array_element))
    (`self.K2_DestroyActor` _asbp_basic_door)))

(fn `FillArray`
  (set `self.DoorWalls` (`|MakeArray` (`self.PossibleDoorPositions`) (`self.PossibleDoorPositions1`) (`self.PossibleDoorPositions2`) (`self.PossibleDoorPositions3`))))

(fn `SetRoomVisibility`
  (params (Visible :type Boolean))
  (bind _returnvalue (select `bool` Visible :`false` "NoCollision" :`true` "QueryAndPhysics" :!type "ECollisionEnabled Enum"))
  (`PrimitiveComponent.SetCollisionEnabled` (`self.Wall1`) _returnvalue)
  (`PrimitiveComponent.SetCollisionEnabled` (`self.Wall3`) _returnvalue)
  (`PrimitiveComponent.SetCollisionEnabled` (`self.Wall2`) _returnvalue)
  (`PrimitiveComponent.SetCollisionEnabled` (`self.Wall`) _returnvalue)
  (`self.SetActorHiddenInGame` (not (`local.Visible`)))
  (for _array_element (`self.Doors`)
    (`self.SetActorHiddenInGame` _array_element (not (`local.Visible`)))
    (`PrimitiveComponent.SetCollisionEnabled` (`/Game/Blueprints/BP_BasicDoor.DoorGFX` _array_element) _returnvalue)))

(fn `SpawnDoors`
  (locals (doorsSpawned :type Integer) (currentWall :type "BoxComponent Object Reference"))
  (bind _currentwall (`local.currentWall`))
  (bind (_returnvalue_x _returnvalue_y _returnvalue_z) (`KismetMathLibrary.BreakVector` (`SceneComponent.K2_GetComponentLocation` (`self.Floor`))))
  (if (not (`self.spawnedDoors`))
    (for _array_element (`self.DoorWalls`)
      (bind _output_get (set `local.currentWall` _array_element))
      (if (> (`KismetArrayLibrary.Array_Length` (`PrimitiveComponent.GetOverlappingActors` _output_get "BP_BasicRoom_C")) 1)
        (`KismetSystemLibrary.PrintString` "Hello")
        (elif (`KismetMathLibrary.RandomBoolWithWeight` 0.6)
          (bind (_origin _boxextent) (`KismetSystemLibrary.GetComponentBounds` _array_element))
          (bind (_returnvalue_x_2 _returnvalue_y_2) (`KismetMathLibrary.BreakVector` (`KismetMathLibrary.RandomPointInBoundingBox` _origin _boxextent)))
          (bind _returnvalue (`|SpawnActorFromClass` "/Game/Blueprints/BP_BasicDoor.BP_BasicDoor_C" (`KismetMathLibrary.MakeTransform` (`KismetMathLibrary.MakeVector` _returnvalue_x_2 _returnvalue_y_2 _returnvalue_z) (`KismetMathLibrary.FindLookAtRotation` (0.0 0.0 0.0) (`SceneComponent.GetForwardVector` _array_element))) "Undefined" "MultiplyWithRoot" null null))
          (if (`KismetArrayLibrary.Array_IsNotEmpty` (`self.GetOverlappingActors` _returnvalue "/Game/Blueprints/BP_BasicDoor.BP_BasicDoor_C"))
            (`self.K2_DestroyActor` _returnvalue)
            (else
              (`self.K2_AttachToActor` _returnvalue self "None" "KeepWorld" "KeepWorld" "KeepWorld" true)
              (`/Game/Blueprints/BP_BasicDoor.BindRoom` _returnvalue self)
              (`KismetArrayLibrary.Array_Add` (`self.Doors`) _returnvalue)
              (set `/Game/Blueprints/BP_BasicDoor.roomCenter` (+ (`SceneComponent.K2_GetComponentLocation` _currentwall) (* (`SceneComponent.GetForwardVector` _currentwall) 500.0)) _returnvalue)
              (`KismetArrayLibrary.Array_RemoveItem` (`self.DoorWalls`) (`local.currentWall`)))))))
    (set `self.spawnedDoors` true)))

(fn `UserConstructionScript`
  (bind (_origin _boxextent) (`KismetSystemLibrary.GetComponentBounds` (`self.Floor`)))
  (set `self.RoomSize` (`KismetMathLibrary.MakeVector2D` (* (.x _boxextent) 2.0) (* (.y _boxextent) 2.0))))