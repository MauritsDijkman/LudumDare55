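; BP_RangedSpider is a ranged spider enemy that adds visual, audio and attack animation feedback to its parent class.
; BeginPlay creates a dynamic mesh material and attaches a looping-style walk sound, which the Stop and GaDoodTyfus (death) overrides pause.
; Damage triggers a timeline that drives the material's HitEffect parameter as a hit flash before calling the parent.
; PlayAnim plays the attack montage.
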(event `self.ReceiveBeginPlay`
  (`parent.ReceiveBeginPlay`)
  (bind _returnvalue (`PrimitiveComponent.CreateDynamicMaterialInstance` (`self.Mesh`) 0 (`PrimitiveComponent.GetMaterial` (`self.Mesh`) 0) "None"))
  (set `self.Mat` _returnvalue)
  (bind _returnvalue_2 (`GameplayStatics.SpawnSoundAttached` "/Game/Audio/SoundEffects/spiderwalk.spiderwalk" (`self.Mesh`) "None" (0.0 0.0 0.0) (struct) "KeepRelativeOffset" false 1.0 1.0 0.0 null null))
  (set `self.Audio` _returnvalue_2))

(event `self.ReceiveTick`
  (params (DeltaSeconds :type "Float (single-precision)"))
  (`parent.ReceiveTick` DeltaSeconds))

(event `HitEffect`
  (bind (_direction _curve) (`Timeline|Curve` :!via `PlayFromStart`)
    (:`Update`
      (`MaterialInstanceDynamic.SetScalarParameterValue` (`self.Mat`) "HitEffect" _curve))))

(fn `Damage`
  (params (Amt :type "Float (double-precision)") (Normal :type "Vector Structure"))
  (returns (Dead :type Boolean))
  (`self.HitEffect`)
  (bind _dead (`parent.Damage` Amt Normal))
  (return _dead))

(fn `GaDoodTyfus`
  (`parent.GaDoodTyfus`)
  (`AudioComponent.SetPaused` (`self.audio`) true))

(fn `PlayAnim`
  (`self.PlayAnimMontage` "/Game/Characters/Spider/AttackAnim_Montage.AttackAnim_Montage"))

(fn `stop`
  (params (dn :type Boolean))
  (`parent.stop` dn)
  (`AudioComponent.SetPaused` (`self.audio`) dn))

(fn `UserConstructionScript`
  (`parent.UserConstructionScript`))